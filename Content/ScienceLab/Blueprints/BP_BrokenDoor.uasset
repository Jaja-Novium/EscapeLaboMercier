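; BP_BrokenDoor is a sliding double lab door that opens while a BP_Body overlaps its Collision component and closes when it leaves.
; The OpenClose timeline plays on begin overlap and reverses on end overlap, with its play rate set to the inverse of PlayRateS at BeginPlay.
; Each update lerps the panels apart along relative Y, with LabDoor03A first moved alongside LabDoor03B, then overridden in the opposite direction.
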(event `self.ReceiveBeginPlay`
  ; DoorOpeningSpeed(s)
  (`TimelineComponent.SetPlayRate` (`self.Open/Close`) (/ 1.0 (`self.PlayRate(s)`))))

(event `self.Collision.OnComponentBeginOverlap`
  (params (OverlappedComponent :type "PrimitiveComponent Object Reference") (OtherActor :type "Actor Object Reference") (OtherComp :type "PrimitiveComponent Object Reference") (OtherBodyIndex :type Integer) (bFromSweep :type Boolean) (SweepResult :type "HitResult Structure (by ref)"))
  (bind _labdoor03a (`self.LabDoor03A`))
  ;[0 0.3281 0] SecurityBreach0X00CF52
  (cast `/Game/EurileneGene/Core/BP_Body` OtherActor)
  (bind (_direction _alpha) (`Timeline|Open/Close` :!label _label)
    (:`Update`
      (`SceneComponent.K2_SetRelativeLocation` _labdoor03a (`KismetMathLibrary.MakeVector` 0.0 (`KismetMathLibrary.Lerp` 0.0 100.0 _alpha)) false false)
      (`SceneComponent.K2_SetRelativeLocation` (`self.LabDoor03B`) (`KismetMathLibrary.MakeVector` 0.0 (`KismetMathLibrary.Lerp` 0.0 100.0 _alpha)) false false)
      (`SceneComponent.K2_SetRelativeLocation` _labdoor03a (`KismetMathLibrary.MakeVector` 0.0 (`KismetMathLibrary.Lerp` 0.0 -100.0 _alpha)) false false))))

(event `self.Collision.OnComponentEndOverlap`
  (params (OverlappedComponent :type "PrimitiveComponent Object Reference") (OtherActor :type "Actor Object Reference") (OtherComp :type "PrimitiveComponent Object Reference") (OtherBodyIndex :type Integer))
  ;[0 0.3281 0] SecurityBreach0X00CF52
  (cast `/Game/EurileneGene/Core/BP_Body` OtherActor)
  (goto _label :!via `Reverse`))

(fn `UserConstructionScript`)