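; Automatic double sliding lab door that opens while a BP_Body is inside its collision volume.
; The OpenCloseDoor timeline slides the two panels apart along local Y, at a play rate derived from DoorOpenSpeedS.
; When the body leaves the volume, the timeline reverses to close the door and every RailingPlatform132_Blueprint in the level runs CheckWorldGravity.
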(event `self.ReceiveBeginPlay`
  ; OpenDoorSpeed(s)
  (`TimelineComponent.SetPlayRate` (`self.Open/CloseDoor`) (/ 1.0 (`self.DoorOpenSpeed(s)`))))

(event `self.Collision.OnComponentBeginOverlap`
  (params (OverlappedComponent :type "PrimitiveComponent Object Reference") (OtherActor :type "Actor Object Reference") (OtherComp :type "PrimitiveComponent Object Reference") (OtherBodyIndex :type Integer) (bFromSweep :type Boolean) (SweepResult :type "HitResult Structure (by ref)"))
  ;[0 0.3281 0] AutoOpenAndColseDoor
  (cast `/Game/EurileneGene/Core/BP_Body` OtherActor)
  (bind (_direction _alpha) (`Timeline|Open/CloseDoor` :!label _label)
    (:`Update`
      (`SceneComponent.K2_SetRelativeLocation` (`self.LabDoor03B`) (`KismetMathLibrary.MakeVector` 0.0 (`KismetMathLibrary.Lerp` 0.0 100.0 _alpha)) false false)
      (`SceneComponent.K2_SetRelativeLocation` (`self.LabDoor03A`) (`KismetMathLibrary.MakeVector` 0.0 (`KismetMathLibrary.Lerp` 0.0 -100.0 _alpha)) false false))))

(event `CloseDoor`
  ;[0 0.3281 0] AutoOpenAndColseDoor
  (goto _label :!via `Reverse`))

(event `self.Collision.OnComponentEndOverlap`
  (params (OverlappedComponent :type "PrimitiveComponent Object Reference") (OtherActor :type "Actor Object Reference") (OtherComp :type "PrimitiveComponent Object Reference") (OtherBodyIndex :type Integer))
  ;[1 0 0] SecurityBreachFixed
  ;;[0 0.3281 0] CheckingDoorOld
  (`|ExecutionSequence`
    (:`then_0`
      (cast `/Game/EurileneGene/Core/BP_Body` OtherActor)
      (`self.CloseDoor`))
    (:`then_1`
      (cast `/Game/EurileneGene/Core/BP_Body` OtherActor)
      (bind _outactors (`GameplayStatics.GetAllActorsOfClass` "/Game/ScienceLab/Blueprints/RailingPlatform132_Blueprint.RailingPlatform132_Blueprint_C"))
      (for _array_element _outactors
        (`/Game/ScienceLab/Blueprints/RailingPlatform132_Blueprint.CheckWorldGravity` _array_element)))))

(fn `UserConstructionScript`)